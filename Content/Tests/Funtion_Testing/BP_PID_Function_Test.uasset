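; Functional test Blueprint that checks the PIDCalculation function against known expected results.
; On the first tick, a DoOnce runs one calculation with fixed gains, time step and target.
; It then compares the output and the Integral and ErrorPrior state variables with hardcoded values, finishing the test as succeeded or failed.
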(event `self.ReceiveStartTest`)

(event `self.ReceiveTick`
  (params (DeltaSeconds :type "Float (single-precision)"))
  (`/Engine/EditorBlueprintResources/StandardMacros.DoOnce` false
    (:`Completed`
      ;[1 1 1] Calculation
      (bind _returnvalue (`PIDControllerFunctionLibrary.PIDCalculation` 1.0 5.0 2.0 2.0 0.0 0.0 10.0 (`self.Integral`) (`self.Error Prior`)))
      ;[1 1 1] Assertion
      (bind _output_get (set `self.PIDOutput` _returnvalue))
      (if (and (== _output_get -90.0) (== (`self.Integral`) -10.0) (== (`self.Error Prior`) -10.0))
        (`self.FinishTest` "Succeeded" "PID Function test succeeded")
        (else
          (`self.FinishTest` "Failed" "PID Function test Failed"))))))

(fn `UserConstructionScript`)