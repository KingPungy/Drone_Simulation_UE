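; Functional test Blueprint for a hover module, built around a Drone and a TestModule actor.
; On test start it disables physics simulation on the drone body and moves the drone to the module's location without sweep.
; It finishes with an error if the move fails, but has no success condition in its graph.
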(event `self.ReceiveStartTest`
  (bind _drone (`self.Drone`))
  (`PrimitiveComponent.SetSimulatePhysics` (`/Game/Characters/Drone/Drone_Class.DroneBody` _drone) false)
  (bind (_sweephitresult _returnvalue) (`self.K2_SetActorLocation` _drone (`self.K2_GetActorLocation` (`self.Test_Module`)) false false))
  (if (not _returnvalue)
    (`self.FinishTest` "Error" "Problem with moving test actor")))

(event `self.ReceiveTick`
  (params (DeltaSeconds :type "Float (single-precision)"))
  (`parent.ReceiveTick` DeltaSeconds))

(fn `UserConstructionScript`
  (`parent.UserConstructionScript`))